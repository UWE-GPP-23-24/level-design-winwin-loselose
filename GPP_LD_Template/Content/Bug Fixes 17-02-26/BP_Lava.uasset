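; BP_Lava is a freezable lava hazard that kills the player on contact unless it is frozen.
; On BeginPlay it gives the mesh a dynamic material, passes it to the freezable component and binds to that component's frozen-changed event.
; Trigger overlap kills the player immediately or, while frozen, stores them until they leave, so unfreezing kills anyone still standing on it.
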(event OnComponentBeginOverlap(Trigger)
  (params (OverlappedComponent :type Primitive%20Component%20Object%20Reference) (OtherActor :type Actor%20Object%20Reference) (OtherComp :type Primitive%20Component%20Object%20Reference) (OtherBodyIndex :type Integer) (bFromSweep :type Boolean) (SweepResult :type Hit%20Result%20Structure%20%28by%20ref%29))
  ;[0.4491 0.8591 1] Check if player collides and then kill the player
  (bind _asbp_player_character (Utilities|Casting|CastToBP_PlayerCharacter OtherActor))
  (if (CallFunction|IsNotFrozen)
    (Default|KillPlayer _asbp_player_character)
    (Development|PrintString "Killing Player")
    (else
      (Variables|Default|SetTempPlayer _asbp_player_character))))

(event OnComponentEndOverlap(Trigger)
  (params (OverlappedComponent :type Primitive%20Component%20Object%20Reference) (OtherActor :type Actor%20Object%20Reference) (OtherComp :type Primitive%20Component%20Object%20Reference) (OtherBodyIndex :type Integer))
  ;[0.4491 0.8591 1] If player leaves the trigger, set it to null
  (Utilities|Casting|CastToBP_PlayerCharacter OtherActor)
  (Variables|Default|SetTempPlayer 0))

(event Custom|OnFrozenChanged
  (params (IsFrozen :type Boolean))
  ;[0.4491 0.8591 1] Bind to on frozen changed
  ;;[0.4491 0.8591 1] If the player is still on the lava when unfrozen then kill them
  (if (and (not IsFrozen) (!= (Variables|Default|GetTempPlayer) 0))
    (Default|KillPlayer (Variables|Default|GetTempPlayer))
    (Variables|Default|SetTempPlayer 0)))

(event EventBeginPlay
  (bind _mesh (Variables|Default|GetMesh))
  (bind _bp_freezablecomponent (Variables|Default|GetBP_FreezableComponent))
  ;[0.4491 0.8591 1] Initialise freeze component
  (bind _returnvalue (Rendering|Material|CreateDynamicMaterialInstance (Rendering|Material|GetMaterial _mesh 0) "None" "None" :!class /Script/Engine.KismetMaterialLibrary))
  (Rendering|Material|SetMaterial _mesh 0 _returnvalue)
  (Default|InitMaterial _bp_freezablecomponent (Utilities|Array|MakeArray _returnvalue))
  (Default|InitFreezeStatus _bp_freezablecomponent)
  ;[0.4491 0.8591 1] Bind to on frozen changed
  (EventDispatchers|BindEventtoOnFrozenChanged _bp_freezablecomponent (delegate Custom|OnFrozenChanged)))

(event EventDestroyed
  ;[0.4491 0.8591 1] Bind to on frozen changed
  (EventDispatchers|UnbindEventfromOnFrozenChanged (Variables|Default|GetBP_FreezableComponent) (delegate Custom|OnFrozenChanged)))

(fn ConstructionScript)

(fn IsNotFrozen
  (return (not (Default|GetIsFrozen (Variables|Default|GetBP_FreezableComponent)))))